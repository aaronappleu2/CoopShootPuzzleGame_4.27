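; Super speed powerup that temporarily boosts the walk speed of the player pawn it activates on.
; OnActivated caches the pawn and sets its CharacterMovement MaxWalkSpeed to 1.5 times GetMaxSpeed.
; OnExpired divides GetMaxSpeed by the same factor if the pawn is still valid, then calls the parent handler.
; No original speed is stored, so both changes depend on the current movement mode's max speed.
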(event `self.OnActivated`
  (params (PlayerPawn :type "SCharacter Object Reference"))
  (bind _returnvalue (`self.GetComponentByClass` PlayerPawn "/Script/Engine.CharacterMovementComponent"))
  (set `self.Player Pawn` PlayerPawn)
  (set `CharacterMovementComponent.MaxWalkSpeed` (* (`MovementComponent.GetMaxSpeed` _returnvalue) 1.5) _returnvalue))

(event `self.OnExpired`
  (bind _player_pawn (`self.Player Pawn`))
  (bind _returnvalue (`self.GetComponentByClass` _player_pawn "/Script/Engine.CharacterMovementComponent"))
  (`/Engine/EditorBlueprintResources/StandardMacros.IsValid` _player_pawn
    (:`Is Valid`
      (set `CharacterMovementComponent.MaxWalkSpeed` (/ (`MovementComponent.GetMaxSpeed` _returnvalue) 1.5) _returnvalue))
    (:`Is Not Valid`
      _))
  (`parent.OnExpired`))

(fn `UserConstructionScript`)