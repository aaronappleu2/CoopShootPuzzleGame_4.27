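; BP_AdvancedAI is an AI character that runs the BT_AdvancedAI behavior tree through its AI controller when play begins.
; It binds to its health component's change event to update a WBP_HealthIndicator_AI widget with current health as a fraction of default health.
; The widget component is hidden once health drops to zero or below.
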(event `self.ReceiveBeginPlay`
  (`AIController.RunBehaviorTree` (`AIBlueprintHelperLibrary.GetAIController` self) "/Game/AdvancedAI/BT_AdvancedAI.BT_AdvancedAI")
  (add `SHealthComponent.OnHealthChanged` (`self.HealthComp`) (delegate `OnHealthChanged_Event_0`)))

(event `OnHealthChanged_Event_0`
  (params (HealthComp :type "SHealthComponent Object Reference") (Health :type "Float (double-precision)") (HealthDelta :type "Float (double-precision)") (DamageType :type "DamageType Object Reference") (InstigatedBy :type "Controller Object Reference") (DamageCauser :type "Actor Object Reference"))
  (bind _widget (`self.Widget`))
  (bind _aswbp_health_indicator_ai (cast `/Game/UI/WBP_HealthIndicator_AI` (`WidgetComponent.GetWidget` _widget)))
  (`/Game/UI/WBP_HealthIndicator_AI.SetProgress` _aswbp_health_indicator_ai (/ Health (`SHealthComponent.DefaultHealth` (`self.HealthComp`))))
  (`SceneComponent.SetVisibility` _widget (not (<= Health 0.0)) false))

(fn `UserConstructionScript`)